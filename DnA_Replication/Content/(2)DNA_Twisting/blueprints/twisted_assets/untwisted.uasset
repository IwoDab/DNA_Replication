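; Actor Blueprint for an untwisted DNA model that moves on timelines and changes material on key input.
; On BeginPlay, two chained timelines drive the Dna component's relative location, one playing forward and the other in reverse, restarting the first to repeat.
; Tick polls for the 1 key, stepping a non-looping MultiGate through two material changes on element 0, so only the first two presses take effect.
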(event `self.ReceiveBeginPlay`
  (bind (_direction _newtrack_0) (`Timeline|Timeline` :!label _label)
    (:`Update`
      (`SceneComponent.K2_SetRelativeLocation` (`self.dna`) _newtrack_0 false false))
    (:`Finished`
      (bind (_direction_2 _newtrack_0_2) (`Timeline|Timeline_0` :!via `Reverse`)
        (:`Update`
          (`SceneComponent.K2_SetRelativeLocation` (`self.dna`) _newtrack_0_2 false false))
        (:`Finished`
          (goto _label :!via `PlayFromStart`))))))

(event `self.ReceiveTick`
  (params (DeltaSeconds :type "Float (single-precision)"))
  (bind _dna (`self.dna`))
  (bind _returnvalue (`InputDeviceLibrary.GetPlayerControllerFromInputDevice` (struct)))
  (if (`PlayerController.WasInputKeyJustPressed` _returnvalue "One")
    (`|MultiGate` false
      (:`Out 0`
        (`PrimitiveComponent.SetMaterial` _dna 0 null))
      (:`Out 1`
        (`PrimitiveComponent.SetMaterial` _dna 0 null)))))

(fn `UserConstructionScript`)