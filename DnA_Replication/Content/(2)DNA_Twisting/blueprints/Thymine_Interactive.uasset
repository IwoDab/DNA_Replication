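; Interactive Thymine base actor for a DNA twisting scene, with an animated position and a switchable material.
; On BeginPlay, two chained timelines drive the Thymine component's relative location: one plays forward, the other is reversed, then the first restarts, forming a loop.
; Tick polls the player controller for the 2 key, and a looping MultiGate alternates the material between T_OFF and T_ON on each press.
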(event `self.ReceiveBeginPlay`
  (bind (_direction _newtrack_0) (`Timeline|Timeline` :!label _label)
    (:`Update`
      (`SceneComponent.K2_SetRelativeLocation` (`self.Thymine`) _newtrack_0 false false))
    (:`Finished`
      (bind (_direction_2 _newtrack_0_2) (`Timeline|Timeline_0` :!via `Reverse`)
        (:`Update`
          (`SceneComponent.K2_SetRelativeLocation` (`self.Thymine`) _newtrack_0_2 false false))
        (:`Finished`
          (goto _label :!via `PlayFromStart`))))))

(event `self.ReceiveTick`
  (params (DeltaSeconds :type "Float (single-precision)"))
  (bind _thymine (`self.Thymine`))
  (bind _returnvalue (`InputDeviceLibrary.GetPlayerControllerFromInputDevice` (struct)))
  (if (`PlayerController.WasInputKeyJustPressed` _returnvalue "Two")
    (`|MultiGate` false true
      (:`Out 0`
        (`PrimitiveComponent.SetMaterial` _thymine 0 "/Game/(2)DNA_Twisting/Materials/T_OFF.T_OFF"))
      (:`Out 1`
        (`PrimitiveComponent.SetMaterial` _thymine 0 "/Game/(2)DNA_Twisting/Materials/T_ON.T_ON")))))

(fn `UserConstructionScript`)