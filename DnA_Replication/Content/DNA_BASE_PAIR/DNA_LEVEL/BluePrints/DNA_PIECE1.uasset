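; DNA piece actor, apparently an adenine base, that moves along timeline-driven paths and can switch its glow material.
; On BeginPlay two timelines drive the mesh's relative location, chained through their Finished events (forward play, then reverse) to loop.
; Tick polls the player controller for the F key, and a looping MultiGate alternates material slot 1 between Adenine and its glow-off variant.
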(event `self.ReceiveBeginPlay`
  (bind (_direction _newtrack_0) (`Timeline|Timeline` :!label _label)
    (:`Update`
      (`SceneComponent.K2_SetRelativeLocation` (`self.dna_piece`) _newtrack_0 false false))
    (:`Finished`
      (bind (_direction_2 _newtrack_0_2) (`Timeline|Timeline_0` :!via `Reverse`)
        (:`Update`
          (`SceneComponent.K2_SetRelativeLocation` (`self.dna_piece`) _newtrack_0_2 false false))
        (:`Finished`
          (goto _label :!via `PlayFromStart`))))))

(event `self.ReceiveTick`
  (params (DeltaSeconds :type "Float (single-precision)"))
  (bind _dna_piece (`self.dna_piece`))
  (bind _returnvalue (`InputDeviceLibrary.GetPlayerControllerFromInputDevice` (struct)))
  (if (`PlayerController.WasInputKeyJustPressed` _returnvalue "F")
    (`|MultiGate` false true
      (:`Out 0`
        (`PrimitiveComponent.SetMaterial` _dna_piece 1 "/Game/DNA_BASE_PAIR/DNA_LEVEL/Materials/Adenine/Adenine.Adenine"))
      (:`Out 1`
        (`PrimitiveComponent.SetMaterial` _dna_piece 1 "/Game/DNA_BASE_PAIR/DNA_LEVEL/Materials/Adenine/Adenine_off_glow.Adenine_off_glow")))))

(fn `UserConstructionScript`)